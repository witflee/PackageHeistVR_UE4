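; A randomized cardboard box prop that motion controllers can pick up and drop.
; Shortly after BeginPlay it randomly destroys itself or takes a quarter-turn yaw with slight jitter and a random box mesh.
; The mesh switch wires seven variants, but its random range only reaches the first five.
; Pickup, called by BP_MotionController, disables physics and attaches the box to the given component, while Drop re-enables physics and detaches it.
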(event `self.ReceiveBeginPlay`
  (bind _staticmeshcomponent (`self.StaticMeshComponent`))
  (`KismetSystemLibrary.Delay` 0.5)
  (if (> (`KismetMathLibrary.RandomInteger` 3) 1)
    (`self.K2_DestroyActor`)
    (else
      (`self.K2_SetActorRelativeRotation` (`KismetMathLibrary.MakeRotator` 0.0 0.0 (+ (`KismetMathLibrary.RandomFloatInRange` -15.0 15.0) (* (`KismetMathLibrary.RandomInteger` 3) 90.0))))
      (switch `int` (`KismetMathLibrary.RandomInteger` 5)
        (:`Default`
          (`StaticMeshComponent.SetStaticMesh` _staticmeshcomponent "/Game/GodotWarehouseGLTF/0_MESH_CardboardBox_07_mesh_.0_MESH_CardboardBox_07_mesh_"))
        (:`0`
          (`StaticMeshComponent.SetStaticMesh` _staticmeshcomponent "/Game/GodotWarehouseGLTF/0_MESH_CardboardBox_01_mesh_.0_MESH_CardboardBox_01_mesh_"))
        (:`1`
          (`StaticMeshComponent.SetStaticMesh` _staticmeshcomponent "/Game/GodotWarehouseGLTF/0_MESH_CardboardBox_02_mesh_.0_MESH_CardboardBox_02_mesh_"))
        (:`2`
          (`StaticMeshComponent.SetStaticMesh` _staticmeshcomponent "/Game/GodotWarehouseGLTF/0_MESH_CardboardBox_03_mesh_.0_MESH_CardboardBox_03_mesh_"))
        (:`3`
          (`StaticMeshComponent.SetStaticMesh` _staticmeshcomponent "/Game/GodotWarehouseGLTF/0_MESH_CardboardBox_04_mesh_.0_MESH_CardboardBox_04_mesh_"))
        (:`4`
          (`StaticMeshComponent.SetStaticMesh` _staticmeshcomponent "/Game/GodotWarehouseGLTF/0_MESH_CardboardBox_05_mesh_.0_MESH_CardboardBox_05_mesh_"))
        (:`5`
          (`StaticMeshComponent.SetStaticMesh` _staticmeshcomponent "/Game/GodotWarehouseGLTF/0_MESH_CardboardBox_06_mesh_.0_MESH_CardboardBox_06_mesh_"))))))

(event `/Game/VirtualRealityBP/Blueprints/PickupActorInterface.Pickup`
  (params (AttachTo :type "SceneComponent Object Reference"))
  (`PrimitiveComponent.SetSimulatePhysics` (`self.StaticMeshComponent`) false)
  (`SceneComponent.K2_AttachToComponent` (`self.K2_GetRootComponent`) AttachTo "None" "KeepWorld" "KeepWorld" "KeepWorld" false))

(event `/Game/VirtualRealityBP/Blueprints/PickupActorInterface.Drop`
  (`PrimitiveComponent.SetSimulatePhysics` (`self.StaticMeshComponent`) true)
  (`self.K2_DetachFromActor` "KeepWorld" "KeepWorld" "KeepWorld"))

(fn `UserConstructionScript`)